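; Player controller for a multiplayer game that handles the end-of-mission screen and pawn respawn requests.
; OnMissionCompleted creates the UI_PlayerGameOver widget and adds it to the viewport, only on the local controller.
; RespawnPawn passes itself and a spawn transform to RespawnRequest on BP_GameMode, which it gets by casting the current game mode.
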(event `self.OnMissionCompleted`
  (params (InstigatorPawn :type "Pawn Object Reference") (bIsMissionSuccess :type Boolean))
  (if (`self.IsLocalController`)
    (bind _returnvalue (`|CreateWidget` "/Game/multi/ui/UI_PlayerGameOver.UI_PlayerGameOver_C" self))
    (`/Engine/EditorBlueprintResources/StandardMacros.IsValid` _returnvalue
      (:`Is Valid`
        (`UserWidget.AddToViewport` _returnvalue 0)))))

(event `RespawnPawn`
  (params (SpawnTransform :type "Transform Structure"))
  (bind _asbp_game_mode (cast `/Game/Blueprints/GameMode/BP_GameMode` (`GameplayStatics.GetGameMode`)))
  (`/Game/Blueprints/GameMode/BP_GameMode.RespawnRequest` _asbp_game_mode self SpawnTransform))

(fn `UserConstructionScript`)